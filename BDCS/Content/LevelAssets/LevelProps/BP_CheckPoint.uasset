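; BP_CheckPoint is a one-time level checkpoint that heals the player and updates their spawn location.
; The first HealCircle overlap passes a DoOnce before the Player tag check, so any actor can consume it.
; For a player, it waits briefly, sends HealMessage, then casts to BP_PlayerCharacter to set the spawn at HealCylinder.
; It then destroys the cylinder and plays an activation sound at the world origin.
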(event `self.HealCircle.OnComponentBeginOverlap`
  (params (OverlappedComponent :type "PrimitiveComponent Object Reference") (OtherActor :type "Actor Object Reference") (OtherComp :type "PrimitiveComponent Object Reference") (OtherBodyIndex :type Integer) (bFromSweep :type Boolean) (SweepResult :type "HitResult Structure (by ref)"))
  (bind _healcylinder (`self.HealCylinder`))
  (`/Engine/EditorBlueprintResources/StandardMacros.DoOnce` false
    (:`Completed`
      (if (`self.ActorHasTag` OtherActor "Player")
        (`KismetSystemLibrary.Delay` 0.3)
        (message `/Game/Blueprints/Interfaces/BPI_Damagable.Heal` OtherActor 200.0)
        (bind _asbp_player_character (cast `/Game/Blueprints/Player/BP_PlayerCharacter` OtherActor))
        (`/Game/Blueprints/Player/BP_PlayerCharacter.Set Spawn Location` _asbp_player_character (`SceneComponent.K2_GetComponentLocation` _healcylinder))
        (`ActorComponent.K2_DestroyComponent` _healcylinder)
        (`GameplayStatics.PlaySoundAtLocation` "/Game/LevelAssets/LevelProps/SFX/CheckPointActivated.CheckPointActivated" (0.0 0.0 0.0) (struct) 1.0 1.0 0.0 null null null null)))))

(fn `UserConstructionScript`)