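; BP_LevelExit is a level exit portal that opens the referenced level when a Player-tagged actor begins overlapping it while it is active.
; Three Activate functions each unhide one sphere, apparently as progress indicators.
; ActivatePortal reveals the portal cylinder, plays a sound at the world origin and sets IsActive.
; Nothing in this Blueprint calls these functions, so activation is left to external callers.
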(event `self.Portal.OnComponentBeginOverlap`
  (params (OverlappedComponent :type "PrimitiveComponent Object Reference") (OtherActor :type "Actor Object Reference") (OtherComp :type "PrimitiveComponent Object Reference") (OtherBodyIndex :type Integer) (bFromSweep :type Boolean) (SweepResult :type "HitResult Structure (by ref)"))
  (if (and (`self.ActorHasTag` OtherActor "Player") (`self.isActive`))
    (`GameplayStatics.OpenLevelBySoftObjectPtr` (`self.Level`))))

(fn `Activate1`
  (`SceneComponent.SetHiddenInGame` (`self.Sphere`) false false))

(fn `Activate2`
  (`SceneComponent.SetHiddenInGame` (`self.Sphere1`) false false))

(fn `Activate3`
  (`SceneComponent.SetHiddenInGame` (`self.Sphere2`) false false))

(fn `ActivatePortal`
  (`SceneComponent.SetHiddenInGame` (`self.PortalCylinder`) false false)
  (`GameplayStatics.PlaySoundAtLocation` "/Engine/EditorSounds/GamePreview/PossessPlayer.PossessPlayer" (0.0 0.0 0.0) (struct) 1.0 1.0 0.0 null null null null)
  (set `self.isActive` true))

(fn `UserConstructionScript`)