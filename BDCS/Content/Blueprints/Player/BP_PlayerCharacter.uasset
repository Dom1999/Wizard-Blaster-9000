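; Player character with a laser-sighted turret, ammo-limited projectiles, flashbangs, a parry shield and a cooldown blink teleport.
; Handles movement and pause input directly, while aim, combat and teleport are events awaiting external calls.
; DamageSystem owns health and gates actions on death and parry state; Tick drains or refills shield energy.
; Parry sphere-traces to message hit actors, teleport respects BlinkBlocker tags, and death respawns a newly possessed character.
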(event `self.ReceiveTick`
  (params (DeltaSeconds :type "Float (single-precision)"))
  (`self.UpdateShieldEnergy` DeltaSeconds))

(event `self.ReceiveBeginPlay`
  (bind _returnvalue (`|CreateWidget` "/Game/Blueprints/UI/W_HUD.W_HUD_C" (`GameplayStatics.GetPlayerController` 0)))
  (bind _output_get (set `self.HUD` _returnvalue))
  (`UserWidget.AddToViewport` _output_get 0)
  (`PrimitiveComponent.SetEnableGravity` (`MovementComponent.UpdatedPrimitive` (`self.CharacterMovement`)) false))

(event `Laser`
  (bind _ns_laserpointer (`self.NS_LaserPointer`))
  (bind _ns_laserpointer_2 (`self.NS_LaserPointer`))
  (bind _returnvalue (`SceneComponent.K2_GetComponentLocation` _ns_laserpointer))
  (bind _outhit (`KismetSystemLibrary.LineTraceSingle` _returnvalue (+ _returnvalue (* (`SceneComponent.GetForwardVector` _ns_laserpointer) 5000.0)) "TraceTypeQuery1"))
  (if (not (`/Game/Blueprints/Structures/BPC_DamageSystem.IsDead` (`self.DamageSystem`)))
    (`FXSystemComponent.SetVectorParameter` _ns_laserpointer_2 "Beam End" (`KismetMathLibrary.MakeVector` (`KismetMathLibrary.Vector_Distance` (`.ImpactPoint` (`GameplayStatics.BreakHitResult` _outhit)) (`self.K2_GetActorLocation`))))
    (else
      (`FXSystemComponent.SetVectorParameter` _ns_laserpointer_2 "Beam End" (0.0 0.0 0.0)))))

(event `Death`
  (bind _returnvalue (`self.K2_GetActorLocation`))
  (`GameplayStatics.SpawnEmitterAtLocation` "/Game/StarterContent/Particles/P_Explosion.P_Explosion" _returnvalue (struct) (4.0 4.0 4.0))
  (`GameplayStatics.PlaySoundAtLocation` "/Game/StarterContent/Audio/Explosion02.Explosion02" _returnvalue (struct) 1.0 1.0 0.0 null null null null)
  (`self.DisableInput` (`GameplayStatics.GetPlayerController` 0))
  (`|ExecutionSequence`
    (:`then_0`
      (`KismetSystemLibrary.Delay` 4.0)
      (bind _returnvalue_2 (`|SpawnActorFromClass` "BP_PlayerCharacter_C" (`KismetMathLibrary.MakeTransform` (`self.Spawn Transform`)) "Undefined" "MultiplyWithRoot" null null))
      (`Controller.Possess` (`GameplayStatics.GetPlayerController` 0) _returnvalue_2))
    (:`then_1`
      (`self.SetActorHiddenInGame` true))))

(event `DamageResponse`
  (params (DamageResponse :type "/Game/Blueprints/Enums/E_DamageResponse Enum" :default "NewEnumerator0")))

(event `EnhancedInput|/Game/Blueprints/Inputs/IA_Movement`
  (params (ActionValue :type "Vector2D Structure") (ElapsedSeconds :type "Float (double-precision)") (TriggeredSeconds :type "Float (double-precision)") (InputAction :type "InputAction Object Reference" :default "/Game/Blueprints/Inputs/IA_Movement.IA_Movement"))
  (bind (_returnvalue_roll _returnvalue_pitch _returnvalue_yaw) (`KismetMathLibrary.BreakRotator` (`self.GetControlRotation`)))
  (bind _returnvalue (`KismetMathLibrary.MakeRotator` 0.0 0.0 _returnvalue_yaw))
  ;[0 0.5922 0.01177] WASD Movement
  (:`Triggered`
    (`|ExecutionSequence`
      (:`then_0`
        (`self.AddMovementInput` (`KismetMathLibrary.GetForwardVector` _returnvalue) ActionValue_Y))
      (:`then_1`
        (`self.AddMovementInput` (`KismetMathLibrary.GetRightVector` _returnvalue) ActionValue_X)))))

(event `/Game/Blueprints/Interfaces/BPI_MouseLook.LookAt`
  (params (Target :type "Vector Structure"))
  (bind (_returnvalue_x _returnvalue_y) (`KismetMathLibrary.BreakVector` (`self.K2_GetActorLocation`)))
  ;[0 0.3095 0.000911] Mouse Look
  (if (and (not (`/Game/Blueprints/Structures/BPC_DamageSystem.IsDead` (`self.DamageSystem`))) (not (`self.IsMenuOpened`)))
    (`SceneComponent.K2_SetRelativeRotation` (`self.Turret`) (`KismetMathLibrary.FindLookAtRotation` (`KismetMathLibrary.MakeVector` _returnvalue_x _returnvalue_y) (`KismetMathLibrary.MakeVector` Target_X Target_Y)) false false))
  (`self.Laser`))

(event `/Game/Blueprints/Interfaces/BPI_Teleport.StartTeleport`
  (params (Target :type "Vector Structure"))
  (if (not (`/Game/Blueprints/Structures/BPC_DamageSystem.IsDead` (`self.DamageSystem`)))
    (`self.IsTeleportCooldwonComplete`
      (:`True`
        (bind _returnvalue (`|SpawnActorFromClass` "/Game/Blueprints/Player/VFX/BP_TP_Indicator.BP_TP_Indicator_C" (`KismetMathLibrary.MakeTransform` Target) "Undefined" "MultiplyWithRoot" null null))
        (set `self.TeleportIndicator` _returnvalue)
        (`GameplayStatics.PlaySoundAtLocation` "/Engine/VREditor/Sounds/UI/Teleport_Mode_Entered.Teleport_Mode_Entered" (`self.K2_GetActorLocation`) (struct) 1.0 1.0 0.0 null null null null)))))

(event `/Game/Blueprints/Interfaces/BPI_Teleport.CompleteTeleport`
  (bind _returnvalue (`KismetSystemLibrary.GetGameTimeInSeconds`))
  (bind _teleportindicator (`self.TeleportIndicator`))
  (bind _teleportindicator_2 (`self.TeleportIndicator`))
  (bind _outhit (`KismetSystemLibrary.LineTraceSingle` (`self.K2_GetActorLocation`) (`self.TeleportLocation`) "TraceTypeQuery1"))
  (bind (_bblockinghit _binitialoverlap _time _distance _location _impactpoint _normal _impactnormal _physmat _hitactor) (`GameplayStatics.BreakHitResult` _outhit))
  (`/Engine/EditorBlueprintResources/StandardMacros.IsValid` _hitactor
    (:`Is Valid`
      _)
    (:`Is Not Valid`
      _))
  (if (and (!= (`self.TeleportLocation`) (0.0 0.0 0.0) :`ErrorTolerance` 1.0) (not (`self.ActorHasTag` _hitactor "BlinkBlocker")))
    (if (not (`/Game/Blueprints/Structures/BPC_DamageSystem.IsDead` (`self.DamageSystem`)))
      (`self.IsTeleportCooldwonComplete`
        (:`True`
          (`|SpawnActorFromClass` "/Game/Blueprints/Player/VFX/BP_TP_Effect.BP_TP_Effect_C" (`self.GetTransform`) "Undefined" "MultiplyWithRoot" null null)
          (`GameplayStatics.PlaySoundAtLocation` "/Engine/VREditor/Sounds/VR_teleport.VR_teleport" (0.0 0.0 0.0) (struct) 1.0 1.0 0.0 null null null null)
          (`self.K2_TeleportTo` (`KismetMathLibrary.MakeVector` (.x (stale `/Game/Blueprints/Interfaces/BPI_Teleport.SetIndicator` Target)) (.y (stale `/Game/Blueprints/Interfaces/BPI_Teleport.SetIndicator` Target))))
          (`/Engine/EditorBlueprintResources/StandardMacros.IsValid` _teleportindicator_2
            (:`Is Valid`
              (`self.K2_DestroyActor` _teleportindicator_2)
              (set `self.TeleportCooldownStartTime` _returnvalue)
              (set `self.TeleportCooldownEndTime` (+ _returnvalue 3.0)))))))
    (else
      (`/Engine/EditorBlueprintResources/StandardMacros.IsValid` _teleportindicator
        (:`Is Valid`
          (`self.K2_DestroyActor` _teleportindicator))))))

(event `/Game/Blueprints/Interfaces/BPI_Teleport.SetIndicator`
  (params (Target :type "Vector Structure"))
  (bind _teleportindicator (`self.TeleportIndicator`))
  (if (not (`/Game/Blueprints/Structures/BPC_DamageSystem.IsDead` (`self.DamageSystem`)))
    (`self.IsTeleportCooldwonComplete`
      (:`True`
        (bind _output_get (set `self.TeleportLocation` Target))
        (`/Engine/EditorBlueprintResources/StandardMacros.IsValid` _teleportindicator
          (:`Is Valid`
            (`SceneComponent.K2_SetWorldLocation` (`Actor.RootComponent` _teleportindicator) _output_get true false)))))))

(event `ToggleShield`
  (params (IsParrying :type Boolean))
  (if IsParrying
    (bind (_direction _shieldscale) (`Timeline|Timeline` :!label _label)
      (:`Update`
        (`SceneComponent.SetRelativeScale3D` (`self.Shield`) (`KismetMathLibrary.MakeVector` _shieldscale _shieldscale _shieldscale))
        (if (>= _shieldscale 1.9)
          (goto _label :!via `Stop`))))
    (else
      (goto _label :!via `Reverse`))))

(event `/Game/Blueprints/Interfaces/BPI_Parry.Parry`
  (bind _returnvalue (`self.K2_GetActorLocation`))
  (bind _shieldenergy (`self.ShieldEnergy`))
  (bind _isparrying (`/Game/Blueprints/Structures/BPC_DamageSystem.IsParrying` (`self.DamageSystem`)))
  ;[1 0 0.01785] Parry
  (if (and (or (and (> _shieldenergy 0.0) (not _isparrying)) (and _isparrying (!= _shieldenergy 0.0))) (not (`/Game/Blueprints/Structures/BPC_DamageSystem.IsDead` (`self.DamageSystem`))))
    (`|ExecutionSequence`
      (:`then_0`
        (`/Engine/EditorBlueprintResources/StandardMacros.DoOnce` false :!label _label_2
          (:`Completed`
            (`self.ToggleShield` true)
            (`GameplayStatics.PlaySoundAtLocation` "/Engine/VREditor/Sounds/UI/Enter_Play.Enter_Play" (0.0 0.0 0.0) (struct) 1.0 1.0 0.0 null null null null))))
      (:`then_1`
        (set `/Game/Blueprints/Structures/BPC_DamageSystem.IsParrying` true (`self.DamageSystem`))
        (bind _outhits (`KismetSystemLibrary.SphereTraceMulti` :`Start` _returnvalue :`End` _returnvalue :`Radius` 100.0 :`TraceChannel` "TraceTypeQuery1" :`DrawTime` 2.0))
        (for _array_element _outhits
          (message `/Game/Blueprints/Interfaces/BPI_Parry.Parry` (`.HitActor` (`GameplayStatics.BreakHitResult` _array_element))))))
    (else
      (`self.ToggleShield` false))))

(event `/Game/Blueprints/Interfaces/BPI_Parry.EndParry`
  ;[1 0 0.01785] Parry
  (`|ExecutionSequence`
    (:`then_0`
      (goto _label_2 :!via `Reset`))
    (:`then_1`
      (bind _output_get (set `/Game/Blueprints/Structures/BPC_DamageSystem.IsParrying` false (`self.DamageSystem`)))
      (`self.ToggleShield` _output_get))))

(event `/Game/Blueprints/Interfaces/BPI_Fire.Fire`
  (if (and (> (`self.Ammo`) 0) (not (`self.IsReloading`)) (not (`/Game/Blueprints/Structures/BPC_DamageSystem.IsDead` (`self.DamageSystem`))))
    (`KismetSystemLibrary.Delay` 0.1)
    (`self.Fire Basic Projectile`)
    (else
      (`/Engine/EditorBlueprintResources/StandardMacros.DoOnce` false :!label _label_3
        (:`Completed`
          (`self.Reload`))))))

(event `/Game/Blueprints/Interfaces/BPI_Fire.Reload`
  (bind _returnvalue (`self.K2_GetActorLocation`))
  (if (not (`/Game/Blueprints/Structures/BPC_DamageSystem.IsDead` (`self.DamageSystem`)))
    (set `self.IsReloading` true)
    (`GameplayStatics.PlaySoundAtLocation` "/Engine/VREditor/Sounds/UI/Click_on_Button.Click_on_Button" _returnvalue (struct) 1.0 1.0 0.0 null null null null)
    (`KismetSystemLibrary.Delay` 1.5)
    (`GameplayStatics.PlaySoundAtLocation` "/Engine/EditorSounds/GamePreview/EndPlayInEditor_Cue.EndPlayInEditor_Cue" _returnvalue (struct) 1.0 1.0 0.0 null null null null)
    (set `self.Ammo` (`self.MaxAmmo`))
    (set `self.GrenadeAmmo` (`self.MaxGrenadeAmmo`))
    (`self.MoveFlashbangsToStartingPosition`)
    (set `self.IsReloading` false)
    (goto _label_3 :!via `Reset`)))

(event `/Game/Blueprints/Interfaces/BPI_Fire.ThrowFlashbang`
  (params (ProjectileVelocity :type "Float (double-precision)") (ThrowLocation :type "Vector Structure"))
  (bind _bp_flashbangfloater2 (`self.BP_FlashbangFloater2`))
  (bind _bp_flashbangfloater1 (`self.BP_FlashbangFloater1`))
  (bind (_returnvalue_location _returnvalue_rotation) (`KismetMathLibrary.BreakTransform` (`SceneComponent.GetRelativeTransform` (`self.FlashbangDirection`))))
  (if (not (`/Game/Blueprints/Structures/BPC_DamageSystem.IsDead` (`self.DamageSystem`)))
    (switch `int` (`self.GrenadeAmmo`)
      (:`1`
        (`KismetSystemLibrary.MoveComponentTo` _bp_flashbangfloater1 _returnvalue_location _returnvalue_rotation false false 0.1)
        (`SceneComponent.SetHiddenInGame` _bp_flashbangfloater1 true false))
      (:`2`
        (`KismetSystemLibrary.MoveComponentTo` _bp_flashbangfloater2 _returnvalue_location _returnvalue_rotation false false 0.1)
        (`SceneComponent.SetHiddenInGame` _bp_flashbangfloater2 true false)))
    (`self.Fire Flashbang Projectile` ProjectileVelocity)))

(event `EnhancedInput|/Game/Blueprints/Inputs/IA_PauseMenu`
  (params (ActionValue :type Boolean) (ElapsedSeconds :type "Float (double-precision)") (TriggeredSeconds :type "Float (double-precision)") (InputAction :type "InputAction Object Reference" :default "/Game/Blueprints/Inputs/IA_PauseMenu.IA_PauseMenu"))
  (bind _returnvalue (`GameplayStatics.GetPlayerController` 0))
  (:`Triggered`
    (if (not (`self.IsMenuOpened`))
      (set `self.IsMenuOpened` true)
      (bind _returnvalue_2 (`|CreateWidget` "/Game/Blueprints/UI/W_PauseMenu.W_PauseMenu_C" _returnvalue))
      (bind _output_get (set `self.Pause Menu` _returnvalue_2))
      (`UserWidget.AddToViewport` _output_get 0)
      (`WidgetBlueprintLibrary.SetInputMode_UIOnlyEx` _returnvalue _output_get)
      (`GameplayStatics.SetGamePaused` true)
      (else
        (set `self.IsMenuOpened` false)
        (`Widget.RemoveFromParent` (`self.Pause Menu`))
        (`WidgetBlueprintLibrary.SetInputMode_GameOnly` _returnvalue)
        (`GameplayStatics.SetGamePaused` false)
        (`GameplayStatics.SetViewportMouseCaptureMode` "CapturePermanently_IncludingInitialMouseDown")))))

(fn `Fire Basic Projectile`
  (bind (_returnvalue_location _returnvalue_rotation _returnvalue_scale) (`KismetMathLibrary.BreakTransform` (`SceneComponent.K2_GetComponentToWorld` (`self.FireDirection`))))
  (`GameplayStatics.PlaySoundAtLocation` "/Game/Blueprints/Player/SFX/PlayerFireSound.PlayerFireSound" _returnvalue_location (struct) 1.0 1.0 0.0 null null null null)
  (bind _returnvalue (`|SpawnActorFromClass` "/Game/Blueprints/Projectiles/BP_PlayerBulletProjectile.BP_PlayerBulletProjectile_C" (`KismetMathLibrary.MakeTransform` _returnvalue_location _returnvalue_rotation _returnvalue_scale) "AdjustIfPossibleButAlwaysSpawn" "MultiplyWithRoot" self 5000.0 (struct) null))
  (bind _result (`/Engine/EditorBlueprintResources/StandardMacros.DecrementInt` (`self.Ammo`))
    (:`  `
      (set `self.Ammo` _result)
      (bind _projectilemovement (`/Game/Blueprints/Projectiles/BP_ProjectileBase.ProjectileMovement` _returnvalue))
      (`ProjectileMovementComponent.SetVelocityInLocalSpace` _projectilemovement (* (`KismetMathLibrary.Normal` (`KismetMathLibrary.Conv_RotatorToVector` _returnvalue_rotation)) (`MovementComponent.GetMaxSpeed` _projectilemovement))))))

(fn `Fire Flashbang Projectile`
  (params (flashbangVelocity :type "Float (double-precision)"))
  (bind _grenadeammo (`self.GrenadeAmmo`))
  (bind (_returnvalue_location _returnvalue_rotation) (`KismetMathLibrary.BreakTransform` (`SceneComponent.K2_GetComponentToWorld` (`self.FlashbangDirection`))))
  (if (> _grenadeammo 0)
    (bind _result (`/Engine/EditorBlueprintResources/StandardMacros.DecrementInt` _grenadeammo)
      (:`  `
        (set `self.GrenadeAmmo` _result)
        (bind _returnvalue (`|SpawnActorFromClass` "/Game/Blueprints/Projectiles/BP_ProjectileFlashBang.BP_ProjectileFlashBang_C" (`KismetMathLibrary.MakeTransform` _returnvalue_location) "AdjustIfPossibleButAlwaysSpawn" "MultiplyWithRoot" self (`KismetMathLibrary.FClamp` (* flashbangVelocity 3.0) 1500.0 2300.0) (struct) null))
        (bind _projectilemovement (`/Game/Blueprints/Projectiles/BP_ProjectileBase.ProjectileMovement` _returnvalue))
        (`ProjectileMovementComponent.SetVelocityInLocalSpace` _projectilemovement (* (`KismetMathLibrary.Normal` (`KismetMathLibrary.Conv_RotatorToVector` _returnvalue_rotation)) (`MovementComponent.GetMaxSpeed` _projectilemovement)))))))

(fn `GetCurrentHealth`
  (returns (Health :type "Float (double-precision)"))
  (return (`/Game/Blueprints/Structures/BPC_DamageSystem.Health` (`self.DamageSystem`))))

(fn `GetMaxHealth`
  (returns (Health :type "Float (double-precision)"))
  (return (`/Game/Blueprints/Structures/BPC_DamageSystem.MaxHealth` (`self.DamageSystem`))))

(fn `Heal`
  (params (Amount :type "Float (double-precision)"))
  (returns (NewHealth :type "Float (double-precision)"))
  (bind _newhealth (`/Game/Blueprints/Structures/BPC_DamageSystem.Heal` (`self.DamageSystem`) Amount))
  (return _newhealth))

(fn `MoveFlashbangsToStartingPosition`
  (bind _floater1_location_location (`KismetMathLibrary.BreakTransform` (`self.Floater1 Location`)))
  (bind _floater2_location_location (`KismetMathLibrary.BreakTransform` (`self.Floater2 Location`)))
  (bind _bp_flashbangfloater2 (`self.BP_FlashbangFloater2`))
  (bind _bp_flashbangfloater1 (`self.BP_FlashbangFloater1`))
  (`|ExecutionSequence`
    (:`then_0`
      (`SceneComponent.K2_SetRelativeLocation` _bp_flashbangfloater1 _floater1_location_location false false)
      (if (`SceneComponent.bHiddenInGame` _bp_flashbangfloater1)
        (`SceneComponent.SetHiddenInGame` _bp_flashbangfloater1 false false)
        (`GameplayStatics.SpawnEmitterAtLocation` "/Game/StarterContent/Particles/P_Explosion.P_Explosion" (`SceneComponent.K2_GetComponentLocation` _bp_flashbangfloater1) (struct) (0.5 0.5 0.5))))
    (:`then_1`
      (`SceneComponent.K2_SetRelativeLocation` _bp_flashbangfloater2 _floater2_location_location false false)
      (if (`SceneComponent.bHiddenInGame` _bp_flashbangfloater2)
        (`SceneComponent.SetHiddenInGame` _bp_flashbangfloater2 false false)
        (`GameplayStatics.SpawnEmitterAtLocation` "/Game/StarterContent/Particles/P_Explosion.P_Explosion" (`SceneComponent.K2_GetComponentLocation` _bp_flashbangfloater2) (struct) (0.5 0.5 0.5))))))

(fn `Set Spawn Location`
  (params (`New Spawn Location` :type "Vector Structure"))
  (set `self.Spawn Transform` `New Spawn Location`))

(fn `TakeDamage`
  (params (DamageInfo :type "/Game/Blueprints/Structures/S_DamageInfo Structure"))
  (returns (WasDamaged :type Boolean))
  (bind _wasdamaged (`/Game/Blueprints/Structures/BPC_DamageSystem.TakeDamage` (`self.DamageSystem`) DamageInfo))
  (if true
    (`GameplayStatics.PlaySoundAtLocation` "/Game/Blueprints/Player/SFX/HitSound.HitSound" (`self.K2_GetActorLocation`) (struct) 1.0 1.0 0.0 null null null null)
    (return _wasdamaged)))

(fn `UpdateShieldEnergy`
  (params (DeltaTime :type "Float (double-precision)"))
  (if (`/Game/Blueprints/Structures/BPC_DamageSystem.IsParrying` (`self.DamageSystem`))
    (set `self.ShieldEnergy` (`KismetMathLibrary.FClamp` (- (`self.ShieldEnergy`) DeltaTime) 0.0 (`self.MaxShieldEnergy`)))
    (else
      (set `self.ShieldEnergy` (`KismetMathLibrary.FClamp` (+ (`self.ShieldEnergy`) DeltaTime) 0.0 (`self.MaxShieldEnergy`))))))

(fn `UserConstructionScript`
  (bind _damagesystem (`self.DamageSystem`))
  (set `self.Floater1 Location` (`SceneComponent.GetRelativeTransform` (`self.BP_FlashbangFloater2`)))
  (set `self.Floater2 Location` (`SceneComponent.GetRelativeTransform` (`self.BP_FlashbangFloater1`)))
  (add `/Game/Blueprints/Structures/BPC_DamageSystem.OnDeath` _damagesystem (`|CreateDelegate` :!event `Death`))
  (add `/Game/Blueprints/Structures/BPC_DamageSystem.Parry` _damagesystem (`|CreateDelegate` :!event `Parry`))
  (add `/Game/Blueprints/Structures/BPC_DamageSystem.DamageResponse` _damagesystem (`|CreateDelegate` :!event `DamageResponse`))
  (set `self.Spawn Transform` (`self.K2_GetActorLocation`)))