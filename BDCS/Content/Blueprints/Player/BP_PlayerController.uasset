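; Player controller for cursor-aimed play that shows the mouse and relays Enhanced Input actions to the player pawn as message calls.
; Each tick it traces under the cursor, sends the flattened hit point as a look-at target and stores it for teleport targeting.
; Parry, teleport, fire, reload and flashbang are forwarded, with flashbang velocity derived from pawn-to-cursor distance.
; An IsTeleportCooldownComplete time-gate macro is defined but unused in the event graph.
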(event `self.ReceiveBeginPlay`
  ;[1 1 1] Set Mouse Cursor Visible
  (set `self.bShowMouseCursor` true))

(event `self.ReceiveTick`
  (params (DeltaSeconds :type "Float (single-precision)"))
  (bind _hitresult (`self.GetHitResultUnderCursorByChannel` "TraceTypeQuery3"))
  ;[1 1 1] Get Mouse Position and trigger look at
  (message `/Game/Blueprints/Interfaces/BPI_MouseLook.LookAt` (`GameplayStatics.GetPlayerPawn` 0) (`KismetMathLibrary.MakeVector` (.x (`.Location` (`GameplayStatics.BreakHitResult` _hitresult))) (.y (`.Location` (`GameplayStatics.BreakHitResult` _hitresult)))))
  (set `self.Hit Result Location` (`KismetMathLibrary.MakeVector` (.x (`.Location` (`GameplayStatics.BreakHitResult` _hitresult))) (.y (`.Location` (`GameplayStatics.BreakHitResult` _hitresult))))))

(event `EnhancedInput|/Game/Blueprints/Inputs/IA_Parry`
  (params (ActionValue :type Boolean) (ElapsedSeconds :type "Float (double-precision)") (TriggeredSeconds :type "Float (double-precision)") (InputAction :type "InputAction Object Reference" :default "/Game/Blueprints/Inputs/IA_Parry.IA_Parry"))
  (bind _returnvalue (`GameplayStatics.GetPlayerPawn` 0))
  (:`Triggered`
    (message `/Game/Blueprints/Interfaces/BPI_Parry.Parry` _returnvalue))
  (:`Completed`
    (message `/Game/Blueprints/Interfaces/BPI_Parry.EndParry` _returnvalue)))

(event `EnhancedInput|/Game/Blueprints/Inputs/IA_Teleport`
  (params (ActionValue :type "Vector2D Structure") (ElapsedSeconds :type "Float (double-precision)") (TriggeredSeconds :type "Float (double-precision)") (InputAction :type "InputAction Object Reference" :default "/Game/Blueprints/Inputs/IA_Teleport.IA_Teleport"))
  (bind _returnvalue (`GameplayStatics.GetPlayerPawn` 0))
  (bind _hit_result_location (`self.Hit Result Location`))
  (:`Triggered`
    (message `/Game/Blueprints/Interfaces/BPI_Teleport.SetIndicator` _returnvalue _hit_result_location))
  (:`Started`
    (message `/Game/Blueprints/Interfaces/BPI_Teleport.StartTeleport` _returnvalue _hit_result_location))
  (:`Completed`
    (message `/Game/Blueprints/Interfaces/BPI_Teleport.CompleteTeleport` _returnvalue)))

(event `EnhancedInput|/Game/Blueprints/Inputs/IA_Fire`
  (params (ActionValue :type Boolean) (ElapsedSeconds :type "Float (double-precision)") (TriggeredSeconds :type "Float (double-precision)") (InputAction :type "InputAction Object Reference" :default "/Game/Blueprints/Inputs/IA_Fire.IA_Fire"))
  (:`Triggered`
    (message `/Game/Blueprints/Interfaces/BPI_Fire.Fire` (`GameplayStatics.GetPlayerPawn` 0))))

(event `EnhancedInput|/Game/Blueprints/Inputs/IA_Reload`
  (params (ActionValue :type Boolean) (ElapsedSeconds :type "Float (double-precision)") (TriggeredSeconds :type "Float (double-precision)") (InputAction :type "InputAction Object Reference" :default "/Game/Blueprints/Inputs/IA_Reload.IA_Reload"))
  (:`Triggered`
    (message `/Game/Blueprints/Interfaces/BPI_Fire.Reload` (`GameplayStatics.GetPlayerPawn` 0))))

(event `EnhancedInput|/Game/Blueprints/Inputs/IA_FlashBang`
  (params (ActionValue :type Boolean) (ElapsedSeconds :type "Float (double-precision)") (TriggeredSeconds :type "Float (double-precision)") (InputAction :type "InputAction Object Reference" :default "/Game/Blueprints/Inputs/IA_FlashBang.IA_FlashBang"))
  (bind _returnvalue (`GameplayStatics.GetPlayerPawn` 0))
  (:`Triggered`
    (message `/Game/Blueprints/Interfaces/BPI_Fire.ThrowFlashbang` _returnvalue (`KismetMathLibrary.Vector_Distance` (`self.K2_GetActorLocation` _returnvalue) (`.Location` (`GameplayStatics.BreakHitResult` (`self.GetHitResultUnderCursorByChannel` "TraceTypeQuery3")))) (0.0 0.0 0.0))))

(fn `UserConstructionScript`)