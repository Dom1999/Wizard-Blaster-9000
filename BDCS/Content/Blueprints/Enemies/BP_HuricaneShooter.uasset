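; BP_HuricaneShooter is a shielded enemy that starts parrying and fires blue grenades at the player.
; On seeing the player it turns toward them, waits a randomized interval, then, unless in a hit reaction, animates and launches a BP_BlueGrenade from FireDirection.
; A Stagger response ends parrying and plays a timeline that scales then destroys the shield, forwarding the response to the parent on every timeline update.
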(event `self.ReceiveBeginPlay`
  (`parent.ReceiveBeginPlay`)
  (set `/Game/Blueprints/Structures/BPC_DamageSystem.IsParrying` true (`self.BPC_DamageSystem`)))

(event `self.OnDamageResponse`
  (params (DamageResponse :type "/Game/Blueprints/Enums/E_DamageResponse Enum" :default "NewEnumerator0"))
  (switch `/Game/Blueprints/Enums/E_DamageResponse` DamageResponse
    (:`NewEnumerator0`
      (`parent.OnDamageResponse` DamageResponse :!label _label))
    (:`NewEnumerator2`
      (set `/Game/Blueprints/Structures/BPC_DamageSystem.IsParrying` false (`self.BPC_DamageSystem`))
      (bind (_direction _shieldscale) (`Timeline|ShieldDestroyTimeline`)
        (:`Update`
          (`SceneComponent.SetWorldScale3D` (`self.Shield`) (`KismetMathLibrary.MakeVector` _shieldscale _shieldscale _shieldscale))
          (goto _label))
        (:`Finished`
          (`ActorComponent.K2_DestroyComponent` (`self.Shield`)))))))

(event `self.ReceiveTick`
  (params (DeltaSeconds :type "Float (single-precision)"))
  (`parent.ReceiveTick` DeltaSeconds))

(event `/Game/Blueprints/Interfaces/BPI_EnemyBehaviour.OnCantSeePlayer`)

(event `/Game/Blueprints/Interfaces/BPI_EnemyBehaviour.OnCanSeePlayer`
  (`self.TurnTowardsTarget` (`self.K2_GetActorLocation` (`GameplayStatics.GetPlayerCharacter` 0)))
  (`self.Attack`))

(event `Attack`
  (bind _attackspeed (`self.AttackSpeed`))
  (bind (_returnvalue_location _returnvalue_rotation _returnvalue_scale) (`KismetMathLibrary.BreakTransform` (`SceneComponent.K2_GetComponentToWorld` (`self.FireDirection`))))
  (`KismetSystemLibrary.Delay` (`KismetMathLibrary.RandomFloatInRange` _attackspeed (+ _attackspeed 2.0)))
  (if (`|EnumEquality` (`self.HitReaction`) "NewEnumerator0")
    (`SkeletalMeshComponent.PlayAnimation` (`self.Mesh`) "/Game/Blueprints/Enemies/EnemyAssets/Animations/AttackAnimation_Anim.AttackAnimation_Anim" false)
    (`KismetSystemLibrary.Delay` 0.5)
    (bind _returnvalue (`|SpawnActorFromClass` "/Game/Blueprints/Projectiles/BP_BlueGrenade.BP_BlueGrenade_C" (`KismetMathLibrary.MakeTransform` _returnvalue_location _returnvalue_rotation _returnvalue_scale) "AdjustIfPossibleButAlwaysSpawn" "MultiplyWithRoot" null 1000.0 (struct) null))
    (bind _projectilemovement (`/Game/Blueprints/Projectiles/BP_ProjectileBase.ProjectileMovement` _returnvalue))
    (`ProjectileMovementComponent.SetVelocityInLocalSpace` _projectilemovement (* (`KismetMathLibrary.Normal` (`KismetMathLibrary.Conv_RotatorToVector` _returnvalue_rotation)) (`MovementComponent.GetMaxSpeed` _projectilemovement)))))

(fn `UserConstructionScript`
  (`parent.UserConstructionScript`))