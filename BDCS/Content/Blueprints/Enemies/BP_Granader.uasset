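; BP_Granader is a grenade-throwing enemy that starts in a parrying state behind a shield.
; On sight it turns to the player, triggers a randomly delayed attack launching BP_GreenGrenade along FireDirection unless hit-reacting, then teleports to a random point around the player after a delay.
; Without sight it wanders to random nearby points.
; A Stagger damage response ends parrying and scales the shield on a timeline before destroying it.
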(event `self.ReceiveBeginPlay`
  (`parent.ReceiveBeginPlay`)
  (set `/Game/Blueprints/Structures/BPC_DamageSystem.IsParrying` true (`self.BPC_DamageSystem`)))

(event `self.OnDamageResponse`
  (params (DamageResponse :type "/Game/Blueprints/Enums/E_DamageResponse Enum" :default "NewEnumerator0"))
  (switch `/Game/Blueprints/Enums/E_DamageResponse` DamageResponse
    (:`NewEnumerator0`
      (`parent.OnDamageResponse` DamageResponse :!label _label))
    (:`NewEnumerator2`
      (set `/Game/Blueprints/Structures/BPC_DamageSystem.IsParrying` false (`self.BPC_DamageSystem`))
      (bind (_direction _shieldscale) (`Timeline|ShieldDestroyTimeline`)
        (:`Update`
          (`SceneComponent.SetWorldScale3D` (`self.Shield`) (`KismetMathLibrary.MakeVector` _shieldscale _shieldscale _shieldscale))
          (goto _label))
        (:`Finished`
          (`ActorComponent.K2_DestroyComponent` (`self.Shield`)))))))

(event `self.ReceiveTick`
  (params (DeltaSeconds :type "Float (single-precision)"))
  (`parent.ReceiveTick` DeltaSeconds))

(event `self.OnCanSeePlayer`
  (bind (_returnvalue_x _returnvalue_y _returnvalue_z) (`KismetMathLibrary.BreakVector` (`SceneComponent.K2_GetComponentLocation` (`Character.CapsuleComponent` (`GameplayStatics.GetPlayerCharacter` 0)))))
  (bind _returnvalue (`KismetMathLibrary.RandomPointInBoundingBox` (`KismetMathLibrary.MakeVector` _returnvalue_x _returnvalue_y _returnvalue_z) (`KismetMathLibrary.MakeVector` 1000.0 1000.0 _returnvalue_z)))
  (`self.TurnTowardsTarget` (`self.K2_GetActorLocation` (`GameplayStatics.GetPlayerCharacter` 0)))
  (`|ExecutionSequence`
    (:`then_0`
      (`self.Attack`))
    (:`then_1`
      (`KismetSystemLibrary.Delay` 6.0)
      (`self.K2_TeleportTo` _returnvalue)
      (`GameplayStatics.PlaySoundAtLocation` "/Engine/VREditor/Sounds/VR_teleport.VR_teleport" _returnvalue (struct) 1.0 1.0 0.0 null null null null))))

(event `self.OnCantSeePlayer`
  (`KismetSystemLibrary.Delay` (`KismetMathLibrary.RandomFloatInRange` 1.0 7.0))
  (`|AIMoveTo` self (`KismetMathLibrary.RandomPointInBoundingBox` (`self.K2_GetActorLocation`) (1000.0 1000.0 1000.0)) null 50.0))

(event `Attack`
  (bind _attackspeed (`self.AttackSpeed`))
  (bind (_returnvalue_location _returnvalue_rotation _returnvalue_scale) (`KismetMathLibrary.BreakTransform` (`SceneComponent.K2_GetComponentToWorld` (`self.FireDirection`))))
  (`KismetSystemLibrary.Delay` (`KismetMathLibrary.RandomFloatInRange` _attackspeed (+ _attackspeed 2.0)))
  (if (`|EnumEquality` (`self.HitReaction`) "NewEnumerator0")
    (`SkeletalMeshComponent.PlayAnimation` (`self.Mesh`) "/Game/Blueprints/Enemies/EnemyAssets/Animations/AttackAnimation_Anim.AttackAnimation_Anim" false)
    (`KismetSystemLibrary.Delay` 0.5)
    (bind _returnvalue (`|SpawnActorFromClass` "/Game/Blueprints/Projectiles/BP_GreenGrenade.BP_GreenGrenade_C" (`KismetMathLibrary.MakeTransform` _returnvalue_location _returnvalue_rotation _returnvalue_scale) "AdjustIfPossibleButAlwaysSpawn" "MultiplyWithRoot" null 1000.0 (struct) null))
    (bind _projectilemovement (`/Game/Blueprints/Projectiles/BP_ProjectileBase.ProjectileMovement` _returnvalue))
    (`ProjectileMovementComponent.SetVelocityInLocalSpace` _projectilemovement (* (`KismetMathLibrary.Normal` (`KismetMathLibrary.Conv_RotatorToVector` _returnvalue_rotation)) (`MovementComponent.GetMaxSpeed` _projectilemovement)))))

(fn `UserConstructionScript`
  (`parent.UserConstructionScript`))