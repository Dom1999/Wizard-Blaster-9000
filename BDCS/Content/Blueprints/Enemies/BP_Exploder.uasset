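; BP_Exploder is an enemy that chases the player and fires volleys of blue shrapnel.
; On seeing the player, it turns, starts an AI move to a randomized stopping distance, and triggers Attack.
; After a randomized AttackSpeed-based delay, Attack checks death and hit-reaction state, then plays its animation and sound.
; It spawns BP_BlueShrapnel at three fire-direction components, launching each along that component's forward vector at max speed.
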(event `/Game/Blueprints/Interfaces/BPI_EnemyBehaviour.OnCantSeePlayer`)

(event `/Game/Blueprints/Interfaces/BPI_EnemyBehaviour.OnCanSeePlayer`
  (bind _returnvalue (`GameplayStatics.GetPlayerCharacter` 0))
  (`self.TurnTowardsTarget` (`self.K2_GetActorLocation` _returnvalue))
  (`|AIMoveTo` self (0.0 0.0 0.0) _returnvalue (`KismetMathLibrary.RandomFloatInRange` 200.0 500.0)
    (:`then`
      (`self.Attack`)
      (`KismetSystemLibrary.Delay` (`KismetMathLibrary.RandomFloatInRange` 0.1 0.5)))))

(event `Attack`
  (bind _attackspeed (`self.AttackSpeed`))
  (bind _result (`/Engine/EditorBlueprintResources/StandardMacros.DecrementFloat` (`KismetMathLibrary.RandomFloatInRange` _attackspeed (+ _attackspeed 3.0)))
    (:`  `
      (`KismetSystemLibrary.Delay` _result)
      (if (and (not (`/Game/Blueprints/Structures/BPC_DamageSystem.IsDead` (`self.BPC_DamageSystem`))) (`|EnumEquality` (`self.HitReaction`) "NewEnumerator0"))
        (`SkeletalMeshComponent.PlayAnimation` (`self.Mesh`) "/Game/Blueprints/Enemies/EnemyAssets/Animations/AttackAnimation_Anim.AttackAnimation_Anim" false)
        (`KismetSystemLibrary.Delay` 0.5)
        (`GameplayStatics.PlaySoundAtLocation` "/Game/Blueprints/Enemies/BasicEnemyAttack.BasicEnemyAttack" (0.0 0.0 0.0) (struct) 1.0 1.0 0.0 null null null null)
        (for _array_element (`|MakeArray` (`self.FireDirection`) (`self.FireDirection1`) (`self.FireDirection2`))
          (bind (_returnvalue_location _returnvalue_rotation _returnvalue_scale) (`KismetMathLibrary.BreakTransform` (`SceneComponent.K2_GetComponentToWorld` _array_element)))
          (bind _returnvalue (`|SpawnActorFromClass` "/Game/Blueprints/Projectiles/BP_BlueShrapnel.BP_BlueShrapnel_C" (`KismetMathLibrary.MakeTransform` _returnvalue_location _returnvalue_rotation _returnvalue_scale) "AlwaysSpawn" "MultiplyWithRoot" null 1000.0 (struct) null))
          (bind _projectilemovement (`/Game/Blueprints/Projectiles/BP_ProjectileBase.ProjectileMovement` _returnvalue))
          (`ProjectileMovementComponent.SetVelocityInLocalSpace` _projectilemovement (* (`KismetMathLibrary.Normal` (`KismetMathLibrary.Conv_RotatorToVector` _returnvalue_rotation)) (`MovementComponent.GetMaxSpeed` _projectilemovement))))))))

(fn `UserConstructionScript`
  (`parent.UserConstructionScript`))