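; Basic ranged enemy that turns toward the player on sight and fires projectiles, building on a parent class's events.
; Seeing the player starts an attack after a randomized AttackSpeed-based delay, skipped if the enemy is dead or not in the required hit-reaction state.
; The attack plays its animation, waits briefly, then plays a sound and spawns BP_EnemyProjectile at FireDirection, setting its velocity to max speed.
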(event `self.ReceiveBeginPlay`
  (`parent.ReceiveBeginPlay`))

(event `/Game/Blueprints/Interfaces/BPI_EnemyBehaviour.OnCanSeePlayer`
  (`self.TurnTowardsTarget` (`self.K2_GetActorLocation` (`GameplayStatics.GetPlayerCharacter` 0)))
  (`self.Attack`)
  (set `self.IsShooting` true))

(event `Attack`
  (bind _attackspeed (`self.AttackSpeed`))
  (bind (_returnvalue_location _returnvalue_rotation _returnvalue_scale) (`KismetMathLibrary.BreakTransform` (`SceneComponent.K2_GetComponentToWorld` (`self.FireDirection`))))
  (`KismetSystemLibrary.Delay` (`KismetMathLibrary.RandomFloatInRange` _attackspeed (+ _attackspeed 0.5)))
  (if (and (not (`/Game/Blueprints/Structures/BPC_DamageSystem.IsDead` (`self.BPC_DamageSystem`))) (`|EnumEquality` (`self.HitReaction`) "NewEnumerator0"))
    (`SkeletalMeshComponent.PlayAnimation` (`self.Mesh`) "/Game/Blueprints/Enemies/EnemyAssets/Animations/AttackAnimation_Anim.AttackAnimation_Anim" false)
    (`KismetSystemLibrary.Delay` 0.5)
    (`GameplayStatics.PlaySoundAtLocation` "/Game/Blueprints/Enemies/BasicEnemyAttack.BasicEnemyAttack" (`self.K2_GetActorLocation`) (struct) 1.0 1.0 0.0 null null null null)
    (bind _returnvalue (`|SpawnActorFromClass` "/Game/Blueprints/Projectiles/BP_EnemyProjectile.BP_EnemyProjectile_C" (`KismetMathLibrary.MakeTransform` _returnvalue_location _returnvalue_rotation _returnvalue_scale) "AdjustIfPossibleButAlwaysSpawn" "MultiplyWithRoot" null 500.0 (struct) null))
    (bind _projectilemovement (`/Game/Blueprints/Projectiles/BP_ProjectileBase.ProjectileMovement` _returnvalue))
    (`ProjectileMovementComponent.SetVelocityInLocalSpace` _projectilemovement (* (`KismetMathLibrary.Normal` (`KismetMathLibrary.Conv_RotatorToVector` _returnvalue_rotation)) (`MovementComponent.GetMaxSpeed` _projectilemovement)))))

(fn `UserConstructionScript`
  (`parent.UserConstructionScript`))