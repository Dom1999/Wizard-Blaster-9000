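; Base enemy Blueprint that floats on a timeline, randomly attaches cosmetic accessories at spawn and can play a teleport-in effect.
; On Tick, delayed line traces set player visibility and call seen/unseen hooks, alongside helpers for turning and AI movement.
; BPCDamageSystem handles damage, with its callbacks driving a stagger reaction that halts movement and a death that ragdolls, usually plays a random sound, then explodes and destroys the actor.
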(event `self.ReceiveBeginPlay`
  (bind _returnvalue (`self.GetTransform`))
  (`|ExecutionSequence`
    (:`then_0`
      (set `self.Names` (`|MakeArray` (`self.HatSocket`) (`self.BeardSocket`) (`self.StaffSocket`) (`self.MoustacheSocket`)))
      (set `self.Meshes` (`|MakeArray` (`self.Hat`) (`self.Beard`) (`self.Staff`) (`self.Moustashe`)))
      (for (_array_element _array_index) (`self.Meshes`)
        (if (`KismetMathLibrary.RandomBoolWithWeight` 0.4)
          (`SceneComponent.K2_AttachToComponent` _array_element (`self.Mesh`) (`|GetArrayItem` (`self.Names`) _array_index) "SnapToTarget" "SnapToTarget" "SnapToTarget" true)
          (`SceneComponent.SetHiddenInGame` _array_element false false)
          (else
            (`ActorComponent.K2_DestroyComponent` _array_element)))))
    (:`then_1`
      (bind (_direction _newtrack_0) (`Timeline|Floating`)
        (:`Update`
          (`SceneComponent.K2_SetRelativeLocation` (`self.Mesh`) (`KismetMathLibrary.MakeVector` 0.0 0.0 _newtrack_0) false false))))
    (:`then_2`
      (if (`self.Play Teleprort Effect`)
        (`|SpawnActorFromClass` "/Game/Blueprints/Player/VFX/BP_TP_Effect.BP_TP_Effect_C" _returnvalue "Undefined" "MultiplyWithRoot" null null)
        (`GameplayStatics.PlaySoundAtLocation` "/Engine/VREditor/Sounds/VR_teleport.VR_teleport" (.location _returnvalue) (struct) 1.0 1.0 0.0 null null null null)))
    (:`then_3`
      (`self.SpawnDefaultController`))))

(event `TurnTowardsTarget`
  (params (Target :type "Vector Structure"))
  (bind (_returnvalue_x _returnvalue_y) (`KismetMathLibrary.BreakVector` (`self.K2_GetActorLocation`)))
  (`self.K2_SetActorRelativeRotation` (`KismetMathLibrary.FindLookAtRotation` (`KismetMathLibrary.MakeVector` _returnvalue_x _returnvalue_y) (`KismetMathLibrary.MakeVector` Target_X Target_Y))))

(event `self.ReceiveTick`
  (params (DeltaSeconds :type "Float (single-precision)"))
  (if (and (not (`/Game/Blueprints/Structures/BPC_DamageSystem.IsDead` (`self.BPC_DamageSystem`))) (`|EnumInequality` (`self.HitReaction`) "NewEnumerator2"))
    (`|ExecutionSequence`
      (:`then_0`
        (`KismetSystemLibrary.Delay` (`KismetMathLibrary.RandomFloatInRange` 0.0 1.0))
        (`self.CheckIfSeePlayer`))
      (:`then_1`
        (if (`self.CanSeePlayer`)
          (`self.OnCanSeePlayer`)
          (else
            (`self.OnCantSeePlayer`)))))))

(event `/Game/Blueprints/Interfaces/BPI_EnemyBehaviour.MoveToPlayer`
  (params (Distance :type "Float (double-precision)"))
  (`|AIMoveTo` self (0.0 0.0 0.0) (`GameplayStatics.GetPlayerCharacter` 0) Distance))

(event `OnDamageResponse`
  (params (DamageResponse :type "/Game/Blueprints/Enums/E_DamageResponse Enum" :default "NewEnumerator0"))
  (bind _returnvalue (`KismetMathLibrary.RandomFloatInRange` 0.0 0.15))
  (bind _output_get (set `self.HitReaction` DamageResponse))
  (switch `/Game/Blueprints/Enums/E_DamageResponse` _output_get
    (:`NewEnumerator0`
      (if (`|EnumEquality` (`self.HitReaction`) "NewEnumerator0")
        (`KismetSystemLibrary.Delay` 0.1)
        (set `self.HitReaction` "NewEnumerator0")
        (goto _label :!via `Reset`)))
    (:`NewEnumerator2`
      (set `self.CanSeePlayer` false)
      (`KismetSystemLibrary.Delay` (`KismetMathLibrary.RandomFloatInRange` 0.0 0.1))
      (`MovementComponent.StopMovementImmediately` (`self.CharacterMovement`))
      (`/Engine/EditorBlueprintResources/StandardMacros.DoOnce` false :!label _label
        (:`Completed`
          (`KismetSystemLibrary.Delay` _returnvalue)
          (`SkeletalMeshComponent.PlayAnimation` (`self.Mesh`) "/Game/Blueprints/Enemies/EnemyAssets/Animations/Flashbang_animation_Anim.Flashbang_animation_Anim" false)
          (`KismetSystemLibrary.Delay` (- 3.0 _returnvalue))
          (set `self.HitReaction` "NewEnumerator0")
          (goto _label :!via `Reset`))))))

(event `OnDeath`
  (bind _mesh (`self.Mesh`))
  (`PrimitiveComponent.SetSimulatePhysics` _mesh true)
  (`self.PlayDeathSound`)
  (`PrimitiveComponent.SetCollisionEnabled` _mesh "PhysicsOnly")
  (`PrimitiveComponent.SetCollisionEnabled` (`self.CapsuleComponent`) "NoCollision")
  (`KismetSystemLibrary.Delay` 1.0)
  (`GameplayStatics.SpawnEmitterAtLocation` "/Game/StarterContent/Particles/P_Explosion.P_Explosion")
  (`self.K2_DestroyActor`))

(event `OnParry`)

(fn `CheckIfSeePlayer`
  (bind _outhit (`KismetSystemLibrary.LineTraceSingleForObjects` :`Start` (`SceneComponent.K2_GetComponentLocation` (`self.FireDirection`)) :`End` (`self.K2_GetActorLocation` (`GameplayStatics.GetPlayerCharacter` 0)) :`ObjectTypes` (`self.LineTraceObjectTypes`) :`DrawTime` 0.5))
  (bind (_bblockinghit _binitialoverlap _time _distance _location _impactpoint _normal _impactnormal _physmat _hitactor) (`GameplayStatics.BreakHitResult` _outhit))
  (set `self.CanSeePlayer` (and (`self.ActorHasTag` _hitactor "Player") (not (`Actor.bHidden` _hitactor)))))

(fn `GetCurrentHealth`
  (returns (Health :type "Float (double-precision)"))
  (return 0.0))

(fn `GetMaxHealth`
  (returns (Health :type "Float (double-precision)"))
  (return 0.0))

(fn `Heal`
  (params (Amount :type "Float (double-precision)"))
  (returns (NewHealth :type "Float (double-precision)"))
  (return 0.0))

(fn `PlayDeathSound`
  (bind _returnvalue (`self.K2_GetActorLocation`))
  (switch `int` (`KismetMathLibrary.RandomIntegerInRange` -1 2)
    (:`0`
      (`GameplayStatics.PlaySoundAtLocation` "/Game/Blueprints/Enemies/Death1.Death1" _returnvalue (struct) 1.0 1.0 0.0 null null null null))
    (:`1`
      (`GameplayStatics.PlaySoundAtLocation` "/Game/Blueprints/Enemies/Death3.Death3" _returnvalue (struct) 1.0 1.0 0.0 null null null null))
    (:`2`
      (`GameplayStatics.PlaySoundAtLocation` "/Game/Blueprints/Enemies/Death2.Death2" _returnvalue (struct) 1.0 1.0 0.0 null null null null))))

(fn `TakeDamage`
  (params (DamageInfo :type "/Game/Blueprints/Structures/S_DamageInfo Structure"))
  (returns (WasDamaged :type Boolean))
  (bind _wasdamaged (`/Game/Blueprints/Structures/BPC_DamageSystem.TakeDamage` (`self.BPC_DamageSystem`) DamageInfo))
  (return _wasdamaged))

(fn `UserConstructionScript`
  (bind _bpc_damagesystem (`self.BPC_DamageSystem`))
  (add `/Game/Blueprints/Structures/BPC_DamageSystem.OnDeath` _bpc_damagesystem (`|CreateDelegate` :!event `OnDeath`))
  (add `/Game/Blueprints/Structures/BPC_DamageSystem.DamageResponse` _bpc_damagesystem (`|CreateDelegate` :!event `OnDamageResponse`)))