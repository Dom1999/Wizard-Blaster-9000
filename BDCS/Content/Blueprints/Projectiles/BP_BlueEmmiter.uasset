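; BP_BlueEmmiter is a timed emitter actor that fires BP_BlueProjectile volleys while it spins and moves vertically.
; A timeline started on BeginPlay drives its yaw and height, then destroys the actor on finish.
; Tick runs through a Delay to set the firing cadence, spawning one projectile from each of two arrows.
; Each shot plays a sound and launches at max speed, passing the arrow's world forward vector to SetVelocityInLocalSpace.
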(event `self.ReceiveTick`
  (params (DeltaSeconds :type "Float (single-precision)"))
  (`KismetSystemLibrary.Delay` 0.3)
  (for _array_element (`|MakeArray` (`self.Arrow1`) (`self.Arrow2`))
    (`self.FireProjectile` _array_element)))

(event `self.ReceiveBeginPlay`
  (bind (_returnvalue_x _returnvalue_y) (`KismetMathLibrary.BreakVector` (`self.K2_GetActorLocation`)))
  (bind (_direction _rotationtrack _elevation_track) (`Timeline|RotationTimeline`)
    (:`Update`
      (`self.K2_SetActorLocation` (`KismetMathLibrary.MakeVector` _returnvalue_x _returnvalue_y _elevation_track))
      (`self.K2_SetActorRotation` (`KismetMathLibrary.MakeRotator` 0.0 0.0 _rotationtrack)))
    (:`Finished`
      (`self.K2_DestroyActor`))))

(fn `FireProjectile`
  (params (DirectionArrow :type "ArrowComponent Object Reference"))
  (bind (_returnvalue_location _returnvalue_rotation) (`KismetMathLibrary.BreakTransform` (`SceneComponent.K2_GetComponentToWorld` DirectionArrow)))
  (`GameplayStatics.PlaySoundAtLocation` "/Game/Blueprints/Enemies/SmallAttack.SmallAttack" (`self.K2_GetActorLocation`) (struct) 1.0 1.0 0.0 null null null null)
  (bind _returnvalue (`|SpawnActorFromClass` "/Game/Blueprints/Projectiles/BP_BlueProjectile.BP_BlueProjectile_C" (`KismetMathLibrary.MakeTransform` _returnvalue_location _returnvalue_rotation) "AdjustIfPossibleButAlwaysSpawn" "MultiplyWithRoot" self 500.0 (struct) null))
  (bind _projectilemovement (`/Game/Blueprints/Projectiles/BP_ProjectileBase.ProjectileMovement` _returnvalue))
  (`ProjectileMovementComponent.SetVelocityInLocalSpace` _projectilemovement (* (`KismetMathLibrary.Normal` (`KismetMathLibrary.Conv_RotatorToVector` _returnvalue_rotation)) (`MovementComponent.GetMaxSpeed` _projectilemovement))))

(fn `UserConstructionScript`)