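; Flashbang projectile that bursts shortly after its box collision hits something, affecting actors around the impact point.
; On hit it spawns an impact emitter, waits briefly, then runs a multi-sphere trace at that point and sends a TakeDamage message to each hit actor.
; A timeline then scales up a sphere component as the flash effect, destroying the projectile once the scale passes a threshold.
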(event `FlashEffect`
  (bind (_direction _shieldscale) (`Timeline|Timeline` :!label _label)
    (:`Update`
      (`SceneComponent.SetWorldScale3D` (`self.Sphere`) (`KismetMathLibrary.MakeVector` _shieldscale _shieldscale _shieldscale))
      (if (>= _shieldscale 10.9)
        (`|ExecutionSequence`
          (:`then_0`
            (goto _label :!via `Stop`))
          (:`then_1`
            (`self.K2_DestroyActor`)))))))

(event `self.boxCollision.OnComponentHit`
  (params (HitComponent :type "PrimitiveComponent Object Reference") (OtherActor :type "Actor Object Reference") (OtherComp :type "PrimitiveComponent Object Reference") (NormalImpulse :type "Vector Structure") (Hit :type "HitResult Structure (by ref)"))
  (bind (_bblockinghit _binitialoverlap _time _distance _location) (`GameplayStatics.BreakHitResult` Hit))
  (`GameplayStatics.SpawnEmitterAtLocation` (`self.ImpactEffect`) _location)
  (`KismetSystemLibrary.Delay` 0.8)
  (bind _outhits (`KismetSystemLibrary.SphereTraceMulti` :`Start` _location :`End` _location :`Radius` 800.0 :`TraceChannel` "TraceTypeQuery4" :`bTraceComplex` true :`DrawTime` 1.0))
  (for _array_element _outhits
    (message `/Game/Blueprints/Interfaces/BPI_Damagable.TakeDamage` (`.HitActor` (`GameplayStatics.BreakHitResult` _array_element)) (`self.DamageInfo`)))
  (`self.FlashEffect`))

(fn `UserConstructionScript`
  (`parent.UserConstructionScript`))