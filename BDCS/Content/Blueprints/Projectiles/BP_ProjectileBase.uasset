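; Base projectile actor that destroys itself on collision or after a fixed lifetime and can be parried back as a player bullet.
; The construction script feeds Speed into the movement component, and any destruction triggers the impact effect and sound.
; Parry works once, spawning a player-owned bullet with high damage along the reversed, flattened velocity, without explicitly destroying the original.
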(event `self.ReceiveBeginPlay`
  (`|ExecutionSequence`
    (:`then_0`
      (`KismetSystemLibrary.Delay` 10.0)
      (`self.K2_DestroyActor`))
    (:`then_1`
      (add `self.OnDestroyed` (delegate `OnDestroyed_Event`)))))

(event `OnDestroyed_Event` :!signature `self.OnDestroyed`
  (params (DestroyedActor :type "Actor Object Reference"))
  (bind _returnvalue (`self.K2_GetActorLocation`))
  (`GameplayStatics.SpawnEmitterAtLocation` (`self.ImpactEffect`) _returnvalue)
  (`GameplayStatics.PlaySoundAtLocation` (`self.ImpactSound`) _returnvalue (struct) 1.0 1.0 0.0 null null null null))

(event `self.boxCollision.OnComponentHit`
  (params (HitComponent :type "PrimitiveComponent Object Reference") (OtherActor :type "Actor Object Reference") (OtherComp :type "PrimitiveComponent Object Reference") (NormalImpulse :type "Vector Structure") (Hit :type "HitResult Structure (by ref)"))
  (`self.K2_DestroyActor`))

(event `/Game/Blueprints/Interfaces/BPI_Parry.Parry`
  (bind (_velocity_x _velocity_y) (`KismetMathLibrary.BreakVector` (`MovementComponent.Velocity` (`self.ProjectileMovement`))))
  (`/Engine/EditorBlueprintResources/StandardMacros.DoOnce` false
    (:`Completed`
      (`GameplayStatics.PlaySoundAtLocation` "/Engine/EditorSounds/GamePreview/PossessPlayer.PossessPlayer" (0.0 0.0 0.0) (struct) 1.0 1.0 0.0 null null null null)
      (bind _returnvalue (`|SpawnActorFromClass` "/Game/Blueprints/Projectiles/BP_PlayerBulletProjectile.BP_PlayerBulletProjectile_C" (`KismetMathLibrary.MakeTransform` (`self.K2_GetActorLocation`)) "AlwaysSpawn" "MultiplyWithRoot" (`GameplayStatics.GetPlayerCharacter` 0) 0.0 (struct) null))
      (set `/Game/Blueprints/Projectiles/BP_PlayerBulletProjectile.Damage` (make `/Game/Blueprints/Structures/S_DamageInfo` 200.0 "NewEnumerator2") _returnvalue)
      (`ProjectileMovementComponent.SetVelocityInLocalSpace` (`/Game/Blueprints/Projectiles/BP_ProjectileBase.ProjectileMovement` _returnvalue) (* (`KismetMathLibrary.Normal` (`KismetMathLibrary.NegateVector` (`KismetMathLibrary.MakeVector` _velocity_x _velocity_y))) 5000.0)))))

(fn `UserConstructionScript`
  (bind _projectilemovement (`self.ProjectileMovement`))
  (bind _speed (`self.Speed`))
  (set `ProjectileMovementComponent.InitialSpeed` _speed _projectilemovement)
  (set `ProjectileMovementComponent.MaxSpeed` _speed _projectilemovement))