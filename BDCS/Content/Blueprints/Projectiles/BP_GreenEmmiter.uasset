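; Short-lived emitter actor that bursts green shrapnel projectiles in a ring, playing an acid grenade sound on spawn.
; BeginPlay runs a DoN-gated delay loop for two FireShrapnel volleys, turning the actor's yaw after each so the second ring fills the first's gaps.
; Each volley calls FireProjectile on eight arrow components, spawning a damage-carrying BP_GreenShrapnelProjectile at max speed.
; The actor destroys itself shortly afterwards.
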(event `FireShrapnel`
  (for _array_element (`|MakeArray` (`self.Arrow1`) (`self.Arrow2`) (`self.Arrow3`) (`self.Arrow4`) (`self.Arrow5`) (`self.Arrow6`) (`self.Arrow7`) (`self.Arrow8`))
    (`self.FireProjectile` _array_element)))

(event `self.ReceiveBeginPlay`
  (bind (_returnvalue_roll _returnvalue_pitch _returnvalue_yaw) (`KismetMathLibrary.BreakRotator` (`self.K2_GetActorRotation`)))
  (`|ExecutionSequence`
    (:`then_0`
      (`/Engine/EditorBlueprintResources/StandardMacros.Do N` 2 :!label _label
        (:`Exit`
          (`KismetSystemLibrary.Delay` 0.1)
          (`self.FireShrapnel`)
          (`self.K2_SetActorRotation` (`KismetMathLibrary.MakeRotator` 0.0 0.0 (+ _returnvalue_yaw 22.5)) true)
          (goto _label))))
    (:`then_1`
      (`GameplayStatics.PlaySoundAtLocation` "/Game/Blueprints/Enemies/AcidGrenade.AcidGrenade" (`self.K2_GetActorLocation`) (struct) 1.0 1.0 0.0 null null null null)
      (`KismetSystemLibrary.Delay` 0.5)
      (`self.K2_DestroyActor`))))

(fn `FireProjectile`
  (params (DirectionArrow :type "ArrowComponent Object Reference"))
  (bind (_returnvalue_location _returnvalue_rotation) (`KismetMathLibrary.BreakTransform` (`SceneComponent.K2_GetComponentToWorld` DirectionArrow)))
  (bind _returnvalue (`|SpawnActorFromClass` "/Game/Blueprints/Projectiles/BP_GreenShrapnelProjectile.BP_GreenShrapnelProjectile_C" (`KismetMathLibrary.MakeTransform` _returnvalue_location _returnvalue_rotation) "AdjustIfPossibleButAlwaysSpawn" "MultiplyWithRoot" self 1000.0 (make `/Game/Blueprints/Structures/S_DamageInfo` 10.0) null))
  (if (`KismetSystemLibrary.IsValid` _returnvalue)
    (bind _projectilemovement (`/Game/Blueprints/Projectiles/BP_ProjectileBase.ProjectileMovement` _returnvalue))
    (`ProjectileMovementComponent.SetVelocityInLocalSpace` _projectilemovement (* (`KismetMathLibrary.Normal` (`KismetMathLibrary.Conv_RotatorToVector` _returnvalue_rotation)) (`MovementComponent.GetMaxSpeed` _projectilemovement)))))

(fn `UserConstructionScript`)