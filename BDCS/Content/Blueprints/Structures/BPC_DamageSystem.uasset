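; BPC_DamageSystem is a damage component that tracks health, death, invincibility and parrying for its owner.
; TakeDamage broadcasts the damage response, then uses the CanBeDamaged macro to branch into applying damage, signalling a parry or doing nothing.
; Lethal damage sets IsDead and calls OnDeath.
; Heal clamps MaxHealth plus Amount, rather than current Health, so any non-negative amount restores full health while alive.
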(fn `Heal`
  (params (Amount :type "Float (double-precision)"))
  (returns (NewHealth :type "Float (double-precision)"))
  (if (not (`self.IsDead`))
    (set `self.Health` (`KismetMathLibrary.FClamp` (+ (`self.MaxHealth`) Amount) 0.0 (`self.MaxHealth`)))
    (return 0.0)))

(fn `TakeDamage`
  (params (DamageInfo :type "/Game/Blueprints/Structures/S_DamageInfo Structure"))
  (returns (WasDamaged :type Boolean))
  (bind (_amount _damageresponse) (break `/Game/Blueprints/Structures/S_DamageInfo` DamageInfo))
  (`self.DamageResponse` _damageresponse)
  (`self.CanBeDamaged`
    (:`DoDamage`
      (bind _output_get (set `self.Health` (- (`self.Health`) _amount)))
      (if (<= _output_get 0.0)
        (set `self.IsDead` true)
        (`self.OnDeath`)
        (return true)))
    (:`Parry`
      (`self.Parry`))
    (:`NoDamage`
      (return false))))